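; BP_Player is a thruster-driven player with a fuel gauge, exposing events to switch thrusters and change fuel.
; ActivateThrust and DeactivateThruster toggle the bottom, left or right thruster component by a direction value, and activation starts a shared thruster sound.
; Tick stops that sound once all thrusters are inactive.
; BeginPlay creates the BPW_Player_HUD widget and fills fuel through ChangeFuel, which clamps the value and updates the fuel bar.
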(event `self.ReceiveBeginPlay`
  ;[1 1 1] Activating HUD and Setting Fuel to 100%
  (bind _returnvalue (`|CreateWidget` "/Game/UI/BPW_Player_HUD.BPW_Player_HUD_C"))
  (bind _output_get (set `self.FuelUI` _returnvalue))
  (`UserWidget.AddToViewport` _output_get 0)
  (`self.ChangeFuel` 1.0))

(event `ActivateThrust`
  (params (Direction :type Integer))
  ;[1 1 1] Activate Thrusters
  (switch `int` Direction
    (:`0`
      (if (not (`ActorComponent.IsActive` (`self.BottomThruster`)))
        (`ActorComponent.Activate` (`self.BottomThruster`) false)
        (if (not (`AudioComponent.IsPlaying` (`self.Audio`))) :!label _label
          (`AudioComponent.Play` (`self.Audio`) 0.0))))
    (:`1`
      (if (not (`ActorComponent.IsActive` (`self.LeftThruster`)))
        (`ActorComponent.Activate` (`self.LeftThruster`) false)
        (goto _label)))
    (:`2`
      (if (not (`ActorComponent.IsActive` (`self.RightThruster`)))
        (`ActorComponent.Activate` (`self.RightThruster`) false)
        (goto _label)))))

(event `DeactivateThruster`
  (params (Direction :type Integer))
  ;[1 1 1] Deactivate Thrusters
  (switch `int` Direction
    (:`0`
      (if (`ActorComponent.IsActive` (`self.BottomThruster`))
        (`ActorComponent.Deactivate` (`self.BottomThruster`))))
    (:`1`
      (if (`ActorComponent.IsActive` (`self.LeftThruster`))
        (`ActorComponent.Deactivate` (`self.LeftThruster`))))
    (:`2`
      (if (`ActorComponent.IsActive` (`self.RightThruster`))
        (`ActorComponent.Deactivate` (`self.RightThruster`))))))

(event `ChangeFuel`
  (params (ChangeValue :type "Float (double-precision)"))
  ;[1 1 1] Update the HUD Fuel Bar
  (bind _output_get (set `self.Fuel` (`KismetMathLibrary.FClamp` (+ ChangeValue (`self.Fuel`)))))
  (`ProgressBar.SetPercent` (`/Game/UI/BPW_Player_HUD.FuelBar` (`self.FuelUI`)) _output_get))

(event `self.ReceiveTick`
  (params (DeltaSeconds :type "Float (single-precision)"))
  (bind _audio (`self.Audio`))
  (if (and (not (`ActorComponent.IsActive` (`self.BottomThruster`))) (not (`ActorComponent.IsActive` (`self.LeftThruster`))) (not (`ActorComponent.IsActive` (`self.RightThruster`))))
    (if (`AudioComponent.IsPlaying` _audio)
      (`AudioComponent.Stop` _audio))))

(fn `UserConstructionScript`)