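; BP_Blackhole is a gravity hazard in a lander game that pulls in physics bodies and kills the player on contact.
; Each tick, it accelerates simulating components within GravityInfluenceRange toward its center, ignoring mass, with linear distance falloff scaled by GravityStrength.
; The pull is weighted more heavily on Y and Z than on X.
; Overlapping the Killzone destroys any BPI_Player actor and triggers GameOverLose on GM_Lander.
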(event `self.ReceiveTick`
  (params (DeltaSeconds :type "Float (single-precision)"))
  (`self.ApplyForces`))

(event `self.Killzone.OnComponentBeginOverlap`
  (params (OverlappedComponent :type "PrimitiveComponent Object Reference") (OtherActor :type "Actor Object Reference") (OtherComp :type "PrimitiveComponent Object Reference") (OtherBodyIndex :type Integer) (bFromSweep :type Boolean) (SweepResult :type "HitResult Structure (by ref)"))
  (if (`KismetSystemLibrary.DoesImplementInterface` OtherActor "/Game/Framework/BPI_Player.BPI_Player_C")
    (`self.K2_DestroyActor` OtherActor)
    (bind _asgm_lander (cast `/Game/Framework/GM_Lander` (`GameplayStatics.GetGameMode`)))
    (`/Game/Framework/GM_Lander.GameOverLose` _asgm_lander)))

(fn `ApplyForces`
  (bind _returnvalue (`self.K2_GetActorLocation`))
  (for _array_element (`PrimitiveComponent.GetOverlappingComponents` (`self.GravityInfluenceRange`))
    (if (`SceneComponent.IsSimulatingPhysics` _array_element "None")
      (bind _returnvalue_2 (`SceneComponent.K2_GetComponentLocation` _array_element))
      (`PrimitiveComponent.AddForce` _array_element (* (`KismetMathLibrary.GetDirectionUnitVector` _returnvalue_2 _returnvalue) (* (- 1.0 (`KismetMathLibrary.FClamp` (/ (`KismetMathLibrary.Vector_Distance` _returnvalue _returnvalue_2) 5000.0))) 500.0) (1.0 5.0 5.0) (`self.GravityStrength`)) "None" true))))

(fn `UserConstructionScript`)