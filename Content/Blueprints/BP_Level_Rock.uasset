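; BP_Level_Rock is a placeable level rock hazard that ends the lander game in a loss when the player hits it.
; The Construction Script sets the RockMesh static mesh from the RockType enum, choosing among entry, generic and cliff rock variants.
; On a component hit, an actor implementing BPI_Player is destroyed and GM_Lander's GameOverLose is called.
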(event `self.RockMesh.OnComponentHit`
  (params (HitComponent :type "PrimitiveComponent Object Reference") (OtherActor :type "Actor Object Reference") (OtherComp :type "PrimitiveComponent Object Reference") (NormalImpulse :type "Vector Structure") (Hit :type "HitResult Structure (by ref)"))
  (if (`KismetSystemLibrary.DoesImplementInterface` OtherActor "/Game/Framework/BPI_Player.BPI_Player_C")
    (`self.K2_DestroyActor` OtherActor)
    (bind _asgm_lander (cast `/Game/Framework/GM_Lander` (`GameplayStatics.GetGameMode`)))
    (`/Game/Framework/GM_Lander.GameOverLose` _asgm_lander)))

(fn `UserConstructionScript`
  (`StaticMeshComponent.SetStaticMesh` (`self.RockMesh`) (select `/Game/Blueprints/ENUM_Rock_Type` (`self.RockType`) :`NewEnumerator0` "/Game/Meshes/DeepElderCaves/Meshes/Props/SM_EntryRock_01.SM_EntryRock_01" :`NewEnumerator1` "/Game/Meshes/DeepElderCaves/Meshes/Props/SM_EntryRock_02.SM_EntryRock_02" :`NewEnumerator2` "/Game/Meshes/DeepElderCaves/Meshes/Props/SM_EntryRock_03.SM_EntryRock_03" :`NewEnumerator3` "/Game/Meshes/DeepElderCaves/Meshes/Props/SM_Generic_Rock_A.SM_Generic_Rock_A" :`NewEnumerator4` "/Game/Meshes/DeepElderCaves/Meshes/Props/SM_Generic_Rock_B.SM_Generic_Rock_B" :`NewEnumerator5` "/Game/Meshes/DeepElderCaves/Meshes/Props/SM_Cliff_05.SM_Cliff_05" :`NewEnumerator6` "/Game/Meshes/DeepElderCaves/Meshes/Props/SM_Cliff_06.SM_Cliff_06" :`NewEnumerator7` "/Game/Meshes/DeepElderCaves/Meshes/Props/SM_Cliff_07.SM_Cliff_07" :!type "StaticMesh Object Reference")))