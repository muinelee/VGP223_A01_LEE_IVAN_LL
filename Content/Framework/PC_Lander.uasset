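; Player controller for a lander game that turns player input into thrust on the BP_Player ship.
; BeginPlay caches the first BP_Player found in the level, and every input checks that reference is valid.
; Up and Right axes add fixed upward and scaled sideways physics forces to the ship's Player component.
; Separate action inputs switch bottom, left and right thruster VFX on and off by index, independently of the forces.
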(event `self.ReceiveBeginPlay`
  ;[1 1 1] Reference Ship
  (bind _outactors (`GameplayStatics.GetAllActorsOfClass` "/Game/Blueprints/BP_Player.BP_Player_C"))
  (set `self.PlayerShip` (`|GetArrayItem` _outactors)))

(event `InputAxis|Up`
  (params (AxisValue :type "Float (single-precision)"))
  (bind _playership (`self.PlayerShip`))
  ;[1 1 1] Input for Direction going Up
  (if (> AxisValue 0.01)
    (`/Engine/EditorBlueprintResources/StandardMacros.IsValid` _playership
      (:`Is Valid`
        (`PrimitiveComponent.AddForce` (`/Game/Blueprints/BP_Player.Player` _playership) (0.0 0.0 10.0) "None" false)))))

(event `InputAxis|Right`
  (params (AxisValue :type "Float (single-precision)"))
  (bind _playership (`self.PlayerShip`))
  ;[1 1 1] Input for Direction going Right/Left
  (if (not (`KismetMathLibrary.NearlyEqual_FloatFloat` AxisValue 0.0 0.01))
    (`/Engine/EditorBlueprintResources/StandardMacros.IsValid` _playership
      (:`Is Valid`
        (`PrimitiveComponent.AddForce` (`/Game/Blueprints/BP_Player.Player` _playership) (`KismetMathLibrary.MakeVector` 0.0 (* AxisValue 1.5)) "None" false)))))

(event `InputAction|BottomThruster`
  (params (Key :type "Key Structure"))
  (bind _playership (`self.PlayerShip`))
  (bind _playership_2 (`self.PlayerShip`))
  ;[1 1 1] VFX for Bottom Thruster (Going Up)
  (:`Pressed`
    (`/Engine/EditorBlueprintResources/StandardMacros.IsValid` _playership
      (:`Is Valid`
        (`/Game/Blueprints/BP_Player.ActivateThrust` _playership 0))))
  (:`Released`
    (`/Engine/EditorBlueprintResources/StandardMacros.IsValid` _playership_2
      (:`Is Valid`
        (`/Game/Blueprints/BP_Player.DeactivateThruster` _playership_2 0)))))

(event `InputAction|LeftThruster`
  (params (Key :type "Key Structure"))
  (bind _playership (`self.PlayerShip`))
  (bind _playership_2 (`self.PlayerShip`))
  ;[1 1 1] VFX for Left Thruster (Going Right)
  (:`Pressed`
    (`/Engine/EditorBlueprintResources/StandardMacros.IsValid` _playership_2
      (:`Is Valid`
        (`/Game/Blueprints/BP_Player.ActivateThrust` _playership_2 1))))
  (:`Released`
    (`/Engine/EditorBlueprintResources/StandardMacros.IsValid` _playership
      (:`Is Valid`
        (`/Game/Blueprints/BP_Player.DeactivateThruster` _playership 1)))))

(event `InputAction|RightThruster`
  (params (Key :type "Key Structure"))
  (bind _playership (`self.PlayerShip`))
  (bind _playership_2 (`self.PlayerShip`))
  ;[1 1 1] VFX for Right Thruster (Going Left)
  (:`Pressed`
    (`/Engine/EditorBlueprintResources/StandardMacros.IsValid` _playership
      (:`Is Valid`
        (`/Game/Blueprints/BP_Player.ActivateThrust` _playership 2))))
  (:`Released`
    (`/Engine/EditorBlueprintResources/StandardMacros.IsValid` _playership_2
      (:`Is Valid`
        (`/Game/Blueprints/BP_Player.DeactivateThruster` _playership_2 2)))))

(fn `UserConstructionScript`)