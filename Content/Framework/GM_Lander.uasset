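; GM_Lander is the game mode for a lander game, handling the win and lose end states.
; BeginPlay hides the cursor and sets game-only input.
; GameOverWin and GameOverLose write a result message to the HUD_Lander text and play a sound.
; After a short delay, each shows its level-complete or game-over widget, restoring the cursor and switching to UI-only input.
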(event `self.ReceiveBeginPlay`
  (bind _returnvalue (`GameplayStatics.GetPlayerController` 0))
  (set `PlayerController.bShowMouseCursor` false _returnvalue)
  (`WidgetBlueprintLibrary.SetInputMode_GameOnly` _returnvalue))

(event `GameOverWin`
  (bind _returnvalue (`GameplayStatics.GetPlayerController` 0))
  (bind _ashud_lander (cast `/Game/Framework/HUD_Lander` (`PlayerController.GetHUD` (`GameplayStatics.GetPlayerController` 0))))
  (`TextBlock.SetText` (`/Game/UI/WBP_Lander_Text.TextBottom` (`/Game/Framework/HUD_Lander.HUD` _ashud_lander)) "You Have Landed!")
  (`GameplayStatics.PlaySound2D` "/Engine/VREditor/Sounds/VR_open.VR_open" 1.0 1.0 0.0 null null)
  (`KismetSystemLibrary.Delay` 2.0)
  (bind _returnvalue_2 (`|CreateWidget` "/Game/UI/WBP_LevelComplete.WBP_LevelComplete_C"))
  (`UserWidget.AddToViewport` _returnvalue_2 0)
  (set `PlayerController.bShowMouseCursor` true _returnvalue)
  (`WidgetBlueprintLibrary.SetInputMode_UIOnlyEx` _returnvalue _returnvalue_2))

(event `GameOverLose`
  (bind _returnvalue (`GameplayStatics.GetPlayerController` 0))
  (bind _ashud_lander (cast `/Game/Framework/HUD_Lander` (`PlayerController.GetHUD` (`GameplayStatics.GetPlayerController` 0))))
  (`TextBlock.SetText` (`/Game/UI/WBP_Lander_Text.TextBottom` (`/Game/Framework/HUD_Lander.HUD` _ashud_lander)) "You Have Been Destroyed!")
  (`GameplayStatics.PlaySound2D` "/Game/Audio/Explosion01.Explosion01" 1.0 1.0 0.0 null null)
  (`KismetSystemLibrary.Delay` 2.0)
  (bind _returnvalue_2 (`|CreateWidget` "/Game/UI/WBP_GameOver.WBP_GameOver_C"))
  (`UserWidget.AddToViewport` _returnvalue_2 0)
  (set `PlayerController.bShowMouseCursor` true _returnvalue)
  (`WidgetBlueprintLibrary.SetInputMode_UIOnlyEx` _returnvalue _returnvalue_2))

(fn `UserConstructionScript`)